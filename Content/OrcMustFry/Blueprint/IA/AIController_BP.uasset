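; AIController_BP is an AI controller for an Orc Must Fry character that starts a test behavior tree on BeginPlay.
; It sets up the BBTest_BP blackboard and runs BTTest_BP.
; It then seeds the blackboard with two fixed positions (Pos, PosBis) and sets Target to the player character for the tree to use.
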(event `self.ReceiveBeginPlay`
  (bind _returnvalue (`AIBlueprintHelperLibrary.GetBlackboard` self))
  (`self.UseBlackboard` "/Game/OrcMustFry/Blueprint/IA/BBTest_BP.BBTest_BP")
  (`self.RunBehaviorTree` "/Game/OrcMustFry/Blueprint/IA/BTTest_BP.BTTest_BP")
  (`BlackboardComponent.SetValueAsVector` _returnvalue "Pos" (0.0 0.0 0.0))
  (`BlackboardComponent.SetValueAsVector` _returnvalue "PosBis" (-1000.0 -1000.0 0.0))
  (`BlackboardComponent.SetValueAsObject` _returnvalue "Target" (`GameplayStatics.GetPlayerCharacter` 0)))

(fn `UserConstructionScript`)